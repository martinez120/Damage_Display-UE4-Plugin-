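; Actor that shows floating damage text through a widget component and removes itself when the animation finishes.
; An Initialize event stores the text, and BeginPlay passes it to the Damage_Text widget.
; BeginPlay also binds a handler to the widget's animation-finished event, and HandleAnimFinished destroys the actor.
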(event `self.ReceiveBeginPlay`
  (bind _asdamage_text (cast `/Damage_Indicator/Damage_Text` (`WidgetComponent.GetUserWidgetObject` (`self.Widget`))))
  (add `/Damage_Indicator/Damage_Text.AnimFinished` _asdamage_text (`|CreateDelegate` :!event `HandleAnimFinished`))
  (`/Damage_Indicator/Damage_Text.Initialize` _asdamage_text (`self.Text`)))

(event `self.Initialize`
  (params (text :type "Text (by ref)"))
  (set `self.Text` text))

(fn `HandleAnimFinished`
  ;[1 1 1] Destroys Actor when animation completes
  (`self.K2_DestroyActor`))

(fn `UserConstructionScript`)